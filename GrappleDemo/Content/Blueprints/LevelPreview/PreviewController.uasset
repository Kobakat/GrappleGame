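; PreviewController is a level preview actor, registered as the preview pawn, that drives HUD presentation when a preview starts and ends.
; On initialize it gets the PlayerHUD, caches its transition bar and reticle, and hands itself to the bar as PreviewPawn.
; Preview start requests a bar fade-in and hides the reticle.
; Preview end calls the bar's FadeOutPosses without re-showing the reticle itself.
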(event `On Initialize`
  (bind _asplayer_hud (cast `/Game/Blueprints/UI/PlayerHUD` (`PlayerController.GetHUD` (`GameplayStatics.GetPlayerController` 0))))
  (set `self.Bars` (`/Game/Blueprints/UI/PlayerHUD.TransitionBar` _asplayer_hud))
  (set `/Game/Blueprints/UI/TransitionBar.PreviewPawn` self (`self.Bars`))
  (set `self.Reticle` (`/Game/Blueprints/UI/PlayerHUD.ReticleRefrence` _asplayer_hud)))

(event `self.OnPreviewStarted`
  (`/Game/Blueprints/UI/TransitionBar.FadeInRequest` (`self.Bars`))
  (`/Game/Blueprints/UI/ReticleWidget.ShowReticle` (`self.Reticle`) false))

(event `self.OnPreviewEnd`
  (`/Game/Blueprints/UI/TransitionBar.FadeOutPosses` (`self.Bars`)))

(fn `UserConstructionScript`)