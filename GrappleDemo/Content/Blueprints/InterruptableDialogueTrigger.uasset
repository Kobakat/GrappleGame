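; Trigger actor that plays a voice dialogue clip for the player pawn and can be interrupted mid-playback.
; Overlap begin requests playback, optionally only once, and overlap end withdraws the request if the clip is neither playing nor played.
; PlaySound starts audio scaled by master and voice volume preferences.
; Finishing marks it played and removes the request, whereas Interrupt just stops it, leaving both untouched.
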(event `self.ReceiveBeginPlay`
  (`AudioComponent.SetSound` (`self.AudioSource`) (`self.DialogueClip`))
  (set `self.HasPlayed` false)
  (set `self.IsPlaying` false))

(event `self.ReceiveActorBeginOverlap`
  (params (OtherActor :type "Actor Object Reference"))
  (cast `PlayerPawn` OtherActor)
  (if (not (or (`self.IsPlaying`) (and (`self.OnlyPlaysOnce`) (`self.HasPlayed`))))
    (`self.RequestPlay`)))

(event `self.ReceiveActorEndOverlap`
  (params (OtherActor :type "Actor Object Reference"))
  (cast `PlayerPawn` OtherActor)
  (if (not (or (`self.IsPlaying`) (`self.HasPlayed`)))
    (`self.RemoveRequest`)))

(event `self.PlaySound`
  (params (Preferences :type "AudioPreferenceData Structure"))
  (`AudioComponent.SetVolumeMultiplier` (`self.AudioSource`) (* (/ Preferences_Master 100.0) (/ Preferences_VoiceSounds 100.0)))
  (`AudioComponent.Play` (`self.AudioSource`) 0.0)
  (set `self.IsPlaying` true))

(event `self.AudioSource.OnAudioFinished`
  (set `self.IsPlaying` false)
  (`self.RemoveRequest`)
  (set `self.HasPlayed` true))

(event `self.Interrupt`
  (`AudioComponent.Stop` (`self.AudioSource`))
  (set `self.IsPlaying` false))

(fn `UserConstructionScript`)