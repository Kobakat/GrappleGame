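; World display that shows a level's saved progress: best time, completion state and five pizza collectibles.
; The construction script gives each spinning collectible its own dynamic material, tinted as not collected.
; On BeginPlay it reads LevelName's progress from GrappleGameInstance, recolors collected pizzas by array index, sets the time text (0:00 above a threshold) and turns the light green or red.
; The Debug graph's progress printout is never run.
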(event `self.ReceiveBeginPlay`
  (bind _lightcomponent (`Light.LightComponent` (`self.Completion Light`)))
  ;[1 1 1] Get the Game Instance
  (bind _asgrapple_game_instance (cast `GrappleGameInstance` (`GameplayStatics.GetGameInstance`)))
  (bind _output_get (set `self.GameInstance` _asgrapple_game_instance))
  (bind _returnvalue (`GrappleGameInstance.GetLevelProgress` _output_get (`self.LevelName`)))
  ;[1 1 1] Check which collectibles are collected
  (`self.Check Collectibles`)
  (`|ExecutionSequence`
    (:`then_0`
      (bind (_stagecompleted _besttime) (break `LevelCompletionData` (`.CompletionData` (break `LevelProgress` _returnvalue))))
      (if (> _besttime 18000.0)
        ;[1 1 1] Set Best time to 0 if no best time
        (`TextRenderComponent.K2_SetText` (`self.BestTime`) (`KismetTextLibrary.Conv_StringToText` (`KismetStringLibrary.Concat_StrStr` "Best time:" "0:00")))
        (else
          (`TextRenderComponent.K2_SetText` (`self.BestTime`) (`KismetTextLibrary.Conv_StringToText` (`KismetStringLibrary.Concat_StrStr` "Best time:" (`KismetStringLibrary.TimeSecondsToString` _besttime)))))))
    (:`then_1`
      ;[1 1 1] Change light when level completed
      (if _stagecompleted
        (`LightComponent.SetLightColor` _lightcomponent (struct :`R` 0.184475 :`G` 1.0 :`B` 0.219526 :`A` 1.0) true)
        (else
          (`LightComponent.SetLightColor` _lightcomponent (struct :`R` 0.846873 :`G` 0.011612 :`B` 0.026241 :`A` 1.0) true))))))

(event `self.ReceiveTick`
  (params (DeltaSeconds :type "Float (single-precision)"))
  (`SceneComponent.K2_AddWorldRotation` (`self.Collectible4`) (`KismetMathLibrary.MakeRotator` 0.0 0.0 (* DeltaSeconds (`self.Speed`))) false false)
  (`SceneComponent.K2_AddWorldRotation` (`self.Collectible5`) (`KismetMathLibrary.MakeRotator` 0.0 0.0 (* DeltaSeconds (`self.Speed`))) false false)
  (`SceneComponent.K2_AddWorldRotation` (`self.Collectible1`) (`KismetMathLibrary.MakeRotator` 0.0 0.0 (* DeltaSeconds (`self.Speed`))) false false)
  (`SceneComponent.K2_AddWorldRotation` (`self.Collectible2`) (`KismetMathLibrary.MakeRotator` 0.0 0.0 (* DeltaSeconds (`self.Speed`))) false false)
  (`SceneComponent.K2_AddWorldRotation` (`self.Collectible3`) (`KismetMathLibrary.MakeRotator` 0.0 0.0 (* DeltaSeconds (`self.Speed`))) false false))

(fn `Check Collectibles`
  (bind _collectedcolor (`self.CollectedColor`))
  (bind _returnvalue (`GrappleGameInstance.GetLevelProgress` (`self.GameInstance`) (`self.LevelName`)))
  (for _array_element (`.CollectionMissions` (break `LevelProgress` _returnvalue))
    (for (_array_element_2 _array_index) (`.CollectedStates` (break `CollectionMissionData` _array_element))
      (switch `int` _array_index
        (:`0`
          (if _array_element_2
            (`MaterialInstanceDynamic.SetVectorParameterValue` (`self.Collectible Dynamic Material`) "IsCollected" _collectedcolor)))
        (:`1`
          (if _array_element_2
            (`MaterialInstanceDynamic.SetVectorParameterValue` (`self.Collectible Dynamic Material 2`) "IsCollected" _collectedcolor)))
        (:`2`
          (if _array_element_2
            (`MaterialInstanceDynamic.SetVectorParameterValue` (`self.Collectible Dynamic Material 3`) "IsCollected" _collectedcolor)))
        (:`3`
          (if _array_element_2
            (`MaterialInstanceDynamic.SetVectorParameterValue` (`self.Collectible Dynamic Material 4`) "IsCollected" _collectedcolor)))
        (:`4`
          (if _array_element_2
            (`MaterialInstanceDynamic.SetVectorParameterValue` (`self.Collectible Dynamic Material 5`) "IsCollected" _collectedcolor)))))))

(fn `Debug`)

(fn `UserConstructionScript`
  (bind _notcollectedcolor (`self.NotCollectedColor`))
  (bind _returnvalue (`KismetMaterialLibrary.CreateDynamicMaterialInstance` "/Game/Art/Meshes/Collectibles/CheesePizza.CheesePizza"))
  (bind _output_get (set `self.Collectible Dynamic Material` _returnvalue))
  (bind _returnvalue_2 (`KismetMaterialLibrary.CreateDynamicMaterialInstance` "/Game/Art/Meshes/Collectibles/PepperoniPizza.PepperoniPizza"))
  (bind _output_get_2 (set `self.Collectible Dynamic Material 2` _returnvalue_2))
  (bind _returnvalue_3 (`KismetMaterialLibrary.CreateDynamicMaterialInstance` "/Game/Art/Meshes/Collectibles/VeggiePizza.VeggiePizza"))
  (bind _output_get_3 (set `self.Collectible Dynamic Material 3` _returnvalue_3))
  (bind _returnvalue_4 (`KismetMaterialLibrary.CreateDynamicMaterialInstance` "/Game/Art/Meshes/Collectibles/DeepDishPizza.DeepDishPizza"))
  (bind _output_get_4 (set `self.Collectible Dynamic Material 4` _returnvalue_4))
  (bind _returnvalue_5 (`KismetMaterialLibrary.CreateDynamicMaterialInstance` "/Game/Art/Meshes/Collectibles/GoldenPizza.GoldenPizza"))
  (bind _output_get_5 (set `self.Collectible Dynamic Material 5` _returnvalue_5))
  (`PrimitiveComponent.SetMaterial` (`self.Collectible1`) 0 _output_get)
  (`PrimitiveComponent.SetMaterial` (`self.Collectible2`) 0 _output_get_2)
  (`PrimitiveComponent.SetMaterial` (`self.Collectible3`) 0 _output_get_3)
  (`PrimitiveComponent.SetMaterial` (`self.Collectible4`) 0 _output_get_4)
  (`PrimitiveComponent.SetMaterial` (`self.Collectible5`) 0 _output_get_5)
  (`MaterialInstanceDynamic.SetVectorParameterValue` (`self.Collectible Dynamic Material`) "IsCollected" _notcollectedcolor)
  (`MaterialInstanceDynamic.SetVectorParameterValue` (`self.Collectible Dynamic Material 2`) "IsCollected" _notcollectedcolor)
  (`MaterialInstanceDynamic.SetVectorParameterValue` (`self.Collectible Dynamic Material 3`) "IsCollected" _notcollectedcolor)
  (`MaterialInstanceDynamic.SetVectorParameterValue` (`self.Collectible Dynamic Material 4`) "IsCollected" _notcollectedcolor)
  (`MaterialInstanceDynamic.SetVectorParameterValue` (`self.Collectible Dynamic Material 5`) "IsCollected" _notcollectedcolor))