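; Base pickup actor that floats, spins and is collected when the player overlaps its trigger.
; Tick drives a sine-wave bob on the float pivot around its starting height, spins the revolution axis, and billboards the aura pivot along the camera-to-aura direction.
; On player overlap it calls the empty OnCollected hook for subclasses to define the effect, then destroys itself.
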(event `self.ReceiveBeginPlay`
  ;[1 1 1] Set the base relative height for the bubble floating
  (set `self.BaseHeight` (.z (`SceneComponent.RelativeLocation` (`self.Float Pivot`)))))

(event `self.ReceiveTick`
  (params (DeltaSeconds :type "Float (single-precision)"))
  ;[1 1 1] Update floating cycle and update position
  (bind _output_get (set `self.CurrentFloatCycle` (+ (* DeltaSeconds (`self.FloatSpeed`)) (`self.CurrentFloatCycle`))))
  (`SceneComponent.K2_SetRelativeLocation` (`self.Float Pivot`) (`KismetMathLibrary.MakeVector` 0.0 0.0 (+ (* (`KismetMathLibrary.DegSin` _output_get) (`self.FloatAmplitude`)) (`self.BaseHeight`))) false false)
  ;[1 1 1] Revolve the pickup item
  (`SceneComponent.K2_AddLocalRotation` (`self.Revolution Axis`) (`KismetMathLibrary.MakeRotator` 0.0 0.0 (* DeltaSeconds (`self.RotationSpeed`))) false false)
  ;[1 1 1] Applies rotation such that the aura is forwards facing to the camera
  (`SceneComponent.K2_SetWorldRotation` (`self.Aura Pivot`) (`KismetMathLibrary.MakeRotationFromAxes` (- (`SceneComponent.K2_GetComponentLocation` (`self.Aura Pivot`)) (`SceneComponent.K2_GetComponentLocation` (`PlayerPawn.camera` (`self.Player`)))) (0.0 0.0 0.0) (0.0 0.0 1.0)) false false))

(event `self.Trigger.OnComponentBeginOverlap`
  (params (OverlappedComponent :type "PrimitiveComponent Object Reference") (OtherActor :type "Actor Object Reference") (OtherComp :type "PrimitiveComponent Object Reference") (OtherBodyIndex :type Integer) (bFromSweep :type Boolean) (SweepResult :type "HitResult Structure (by ref)"))
  (bind _player (`self.Player`))
  ;[1 1 1] Do something when the pickup is collected (subclass specified), then destroy
  (if (== OtherActor _player)
    (`self.OnCollected` _player)
    (`self.K2_DestroyActor`)))

(fn `OnCollected`
  (params (Player :type "PlayerPawn Object Reference")))

(fn `UserConstructionScript`)