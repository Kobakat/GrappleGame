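; A pizza collectible pickup that counts toward a collection mission in a game stage, with its collected state persisted in the level progress.
; On BeginPlay it reads that progress from GrappleGameInstance and destroys itself if its mission and collectible index is already marked collected.
; On collection it marks its index, recomputes whether the whole mission is complete, and writes the rebuilt progress back before calling the parent logic.
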(event `self.ReceiveBeginPlay`
  ;[1 1 1] Get the game instance
  (bind _asgrapple_game_instance (cast `GrappleGameInstance` (`GameplayStatics.GetGameInstance`))
    (:`then`
      (bind _output_get (set `self.GameInstance` _asgrapple_game_instance))
      ;[1 1 1] If this collectible has save data for being collected do not spawn it
      (bind _returnvalue (`GrappleGameInstance.GetLevelProgress` _output_get (`self.GameStage`)))
      (if (`|GetArrayItem` (`.CollectedStates` (break `CollectionMissionData` (`|GetArrayItem` (`.CollectionMissions` (break `LevelProgress` _returnvalue)) (`self.MissionIndex`)))) (`self.CollectibleIndex`))
        (`self.K2_DestroyActor`)))
    (:`CastFailed`
      _))
  (`parent.ReceiveBeginPlay`))

(fn `OnCollected`
  (params (Player :type "PlayerPawn Object Reference"))
  (bind _gamestage (`self.GameStage`))
  (bind _gameinstance (`self.GameInstance`))
  (bind _missionindex (`self.MissionIndex`))
  (bind _returnvalue (`GrappleGameInstance.GetLevelProgress` _gameinstance _gamestage))
  (bind (_completiondata _collectionmissions) (break `LevelProgress` _returnvalue))
  (bind _output_get (set `self.CollectionMissionData` (`|GetArrayItem` _collectionmissions _missionindex)))
  (bind (_allarecollected _collectedstates) (break `CollectionMissionData` _output_get))
  (`KismetArrayLibrary.Array_Set` _collectedstates (`self.CollectibleIndex`) true)
  (set `self.AllPickupsComplete` true)
  (for _array_element _collectedstates
    (if (not _array_element)
      (set `self.AllPickupsComplete` false)
      (break)))
  (bind _output_get_2 (set `self.CollectionMissionData` (make `CollectionMissionData` (`self.AllPickupsComplete`) _collectedstates)))
  (`KismetArrayLibrary.Array_Set` _collectionmissions _missionindex _output_get_2)
  (`GrappleGameInstance.SetLevelProgress` _gameinstance (make `LevelProgress` _completiondata _collectionmissions) _gamestage)
  (`parent.OnCollected` null))

(fn `UserConstructionScript`
  (`parent.UserConstructionScript`))