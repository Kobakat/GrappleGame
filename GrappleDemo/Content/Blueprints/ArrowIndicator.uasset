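; ArrowIndicator is an actor whose arrow component is turned toward a TargetPosition, apparently as a direction indicator for the player.
; Each tick it casts player 0's pawn to NewPlayer and stores the camera's forward vector, not its location, as PlayerPosition.
; It sets the arrow's world rotation from TargetPosition minus that vector, with Z zeroed to keep it horizontal.
; A relative-rotation variant is left unconnected.
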(event `self.ReceiveTick`
  (params (DeltaSeconds :type "Float (single-precision)"))
  (bind _asnew_player (cast `/Game/Blueprints/NewPlayer` (`GameplayStatics.GetPlayerPawn` 0)))
  (bind _output_get (set `self.PlayerPosition` (`SceneComponent.GetForwardVector` (`PlayerPawn.camera` _asnew_player))))
  (bind (_returnvalue_x _returnvalue_y) (`KismetMathLibrary.BreakVector` (- (`self.TargetPosition`) _output_get)))
  (`SceneComponent.K2_SetWorldRotation` (`self.Arrow`) (`KismetMathLibrary.Conv_VectorToRotator` (`KismetMathLibrary.MakeVector` _returnvalue_x _returnvalue_y)) false false))

(fn `UserConstructionScript`)