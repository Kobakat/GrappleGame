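; BP_OutOfBounds is an out-of-bounds volume that returns the player to the last checkpoint.
; Both begin and end overlap events on its Trigger component share one respawn path when the overlapping actor is the player pawn.
; That path teleports the pawn to the CPManager's CurrentCheckpoint location, then zeroes the NewPlayer Collider's physics linear velocity so momentum does not carry over.
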(event `self.ReceiveTick`
  (params (DeltaSeconds :type "Float (single-precision)")))

(event `self.ReceiveBeginPlay`)

(event `self.Trigger.OnComponentBeginOverlap`
  (params (OverlappedComponent :type "PrimitiveComponent Object Reference") (OtherActor :type "Actor Object Reference") (OtherComp :type "PrimitiveComponent Object Reference") (OtherBodyIndex :type Integer) (bFromSweep :type Boolean) (SweepResult :type "HitResult Structure (by ref)"))
  (bind _returnvalue (`GameplayStatics.GetPlayerPawn` 0))
  ;[1 1 1] Checks if the player touches the Floor Trigger
  (if (== OtherActor _returnvalue)
    ;[1 1 1] Teleports the player to the last checkpoint it was in
    (`self.K2_SetActorLocation` _returnvalue (`self.K2_GetActorLocation` (`CheckpointManager.currentCheckpoint` (`self.CPManager`))) false true :!label _label)
    (bind _asnew_player (cast `/Game/Blueprints/NewPlayer` _returnvalue))
    (`PrimitiveComponent.SetPhysicsLinearVelocity` (`PlayerPawn.collider` _asnew_player) (0.0 0.0 0.0) false "None")))

(event `self.Trigger.OnComponentEndOverlap`
  (params (OverlappedComponent :type "PrimitiveComponent Object Reference") (OtherActor :type "Actor Object Reference") (OtherComp :type "PrimitiveComponent Object Reference") (OtherBodyIndex :type Integer))
  ;[1 1 1] Check if the player has left the BoxBounds
  (if (== OtherActor (`GameplayStatics.GetPlayerPawn` 0))
    (goto _label)))

(fn `UserConstructionScript`)