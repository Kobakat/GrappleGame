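; ArrowIndicator is a Blueprint that rotates an arrow to show the direction of the next checkpoint relative to the player's view.
; Each Tick it reads NextCheckpoint from the CheckpointManager and, if valid, gets the NewPlayer pawn's camera.
; It sets the arrow's world yaw to the heading angle toward the checkpoint minus the camera's forward heading, ignoring pitch.
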(event `self.ReceiveTick`
  (params (DeltaSeconds :type "Float (single-precision)"))
  (bind _nextcheckpoint (`CheckpointManager.nextCheckpoint` (`self.Checkpoint Manager`)))
  (`/Engine/EditorBlueprintResources/StandardMacros.IsValid` _nextcheckpoint
    (:`Is Valid`
      (set `self.TargetPosition` (`self.K2_GetActorLocation` _nextcheckpoint))
      (bind _asnew_player (cast `/Game/Blueprints/NewPlayer` (`GameplayStatics.GetPlayerPawn` 0)))
      (bind _camera (`PlayerPawn.camera` _asnew_player))
      (bind _returnvalue_location (`KismetMathLibrary.BreakTransform` (`SceneComponent.K2_GetComponentToWorld` _camera)))
      (`SceneComponent.K2_SetWorldRotation` (`self.Arrow`) (`KismetMathLibrary.RotatorFromAxisAndAngle` (0.0 0.0 1.0) (`KismetMathLibrary.RadiansToDegrees` (- (`KismetMathLibrary.Vector_HeadingAngle` (- (`self.TargetPosition`) _returnvalue_location)) (`KismetMathLibrary.Vector_HeadingAngle` (`SceneComponent.GetForwardVector` _camera))))) false false))))

(fn `UserConstructionScript`)