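; A lever reactor Blueprint that sets the direction of a movement track from a switch state.
; On the switched event it keeps the magnitude of the track's current speed, making it positive when the state is true and negative otherwise.
; It then passes the event to its parent, and its construction script only calls the parent version.
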(event `self.ReceiveOnSwitched`
  (params (switchState :type Boolean))
  (bind _movement_track (`self.Movement Track`))
  (bind _returnvalue (`KismetMathLibrary.Abs` (`MovementTrack.currentSpeed` (`self.Movement Track`))))
  ;[1 1 1] Flip the track speed based on the switch state
  (if switchState
    (set `MovementTrack.currentSpeed` _returnvalue _movement_track)
    (else
      (set `MovementTrack.currentSpeed` (* -1.0 _returnvalue) _movement_track)))
  (`parent.ReceiveOnSwitched` switchState))

(fn `UserConstructionScript`
  (`parent.UserConstructionScript`))