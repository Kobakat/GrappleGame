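; Timed button reactor that opens a garage door on activation and lowers it as the timer runs down.
; Activation swaps the cube's material and snaps the door to its open height, while deactivation only swaps the material.
; Each timer tick sets the door's Z by lerping from closed to open with the normalized time remaining, keeping X and Y unchanged.
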(event `self.ReceiveBeginPlay`
  (`PrimitiveComponent.SetMaterial` (`self.Cube`) 0 "/Game/Art/Materials/DarkRed.DarkRed"))

(event `self.ReceiveOnActivated`
  (bind _garage_door (`self.Garage Door`))
  ;[1 1 1] Change button visual
  (`PrimitiveComponent.SetMaterial` (`self.Cube`) 0 (`self.Activated Material`))
  ;[1 1 1] Set initial garage door position
  (`self.K2_SetActorLocation` _garage_door (`KismetMathLibrary.MakeVector` (.x (`self.K2_GetActorLocation` _garage_door)) (.y (`self.K2_GetActorLocation` _garage_door)) (`self.OpenZ`)) false false))

(event `self.ReceiveOnDeactivated`
  ;[1 1 1] Change button visual
  (`PrimitiveComponent.SetMaterial` (`self.Cube`) 0 (`self.Deactivated Material`)))

(event `self.ReceiveOnTimerTick`
  (params (timeRemaining01 :type "Float (single-precision)") (timeRemainingSeconds :type "Float (single-precision)"))
  (bind _garage_door (`self.Garage Door`))
  ;[1 1 1] Animate the garage door
  (`self.K2_SetActorLocation` _garage_door (`KismetMathLibrary.MakeVector` (.x (`self.K2_GetActorLocation` _garage_door)) (.y (`self.K2_GetActorLocation` _garage_door)) (`KismetMathLibrary.Lerp` (`self.ClosedZ`) (`self.OpenZ`) timeRemaining01)) false false))

(fn `UserConstructionScript`)