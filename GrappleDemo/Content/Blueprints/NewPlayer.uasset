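; NewPlayer is a player Blueprint with a grapple gun, whose mesh and hook components are wired up in the Construction Script.
; A dynamic material on the gun mesh shows grapple slack, updated each Tick from the rope length normalized between the gun's min and max.
; Grapple events play shoot and reel sounds.
; A footstep sound event exists, but its movement-driven timer and a jump-prep sound are disconnected.
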(event `self.ReceiveBeginPlay`
  (bind _returnvalue (`PrimitiveComponent.CreateDynamicMaterialInstance` (`self.Gun Mesh`) 1 "/Game/Art/Materials/MAT_GrappleSlack.MAT_GrappleSlack" "None"))
  (set `self.SlackInstance` _returnvalue))

(event `self.ReceiveTick`
  (params (DeltaSeconds :type "Float (single-precision)"))
  (bind _grapplegun (`self.GrappleGun`))
  (bind _minlength (`GrappleGunComponent.MinLength` _grapplegun))
  (bind _returnvalue (`GrappleGunComponent.GetLength` _grapplegun))
  (`MaterialInstanceDynamic.SetScalarParameterValue` (`self.SlackInstance`) "SubtractScalar" (`KismetMathLibrary.FClamp` (/ (- _returnvalue _minlength) (- (`GrappleGunComponent.MaxLength` _grapplegun) _minlength)))))

(event `PlayFootstepSound`
  (`GameplayStatics.PlaySoundAtLocation` "/Game/Sound/sfx_footstep_concrete_Cue.sfx_footstep_concrete_Cue" (- (`self.K2_GetActorLocation`) (0.0 0.0 44.0)) (struct) 1.0 1.0 0.0 null null null))

(event `self.GrappleGun.OnGrappleShot`
  (`GameplayStatics.PlaySound2D` "/Game/Sound/sfx_grappleShoot.sfx_grappleShoot" 1.0 1.0 0.0 null null))

(event `self.GrappleGun.OnGrappleHit`)

(event `self.GrappleGun.OnGrappleStartedTraveling`)

(event `self.GrappleGun.OnGrappleStoppedTraveling`
  (`GameplayStatics.PlaySound2D` "/Game/Sound/sfx_grappleReel.sfx_grappleReel" 1.0 1.0 0.0 null null))

(fn `UserConstructionScript`
  (bind _grapplegun (`self.GrappleGun`))
  (set `self.gun` (`self.Gun Mesh`))
  (set `GrappleGunComponent.GrappleHookEnd` (`self.HookMesh`) _grapplegun)
  (set `GrappleGunComponent.GunEnd` (`self.Gun End`) _grapplegun))